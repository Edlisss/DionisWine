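; Pawn that lets the player drag Bottle actors with the mouse while GrabMode is on, in what appears to be a pouring game.
; Left press traces under the cursor, flags the bottle as moved and starts a looping Grabtick timer on movable hits.
; Grabtick repositions the component along the cursor ray and calls BottleMoving, unless the bottle is pouring.
; Its PhysicsHandle move branch is hard-disabled; release drops the component without clearing the timer.
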(event Custom|Grabtick
  (bind _returnvalue (Game|GetPlayerController 0))
  (bind _grabedcomponent (Variables|Default|GetGrabedComponent))
  (bind _originaldistancetoobject (Variables|Default|GetOriginalDistanceToObject))
  (bind (_worldlocation _worlddirection) (Game|Player|ConvertMouseLocationToWorldSpace _returnvalue))
  (bind _returnvalue_2 (- _originaldistancetoobject 1e+02))
  (bind (_x _y) (Math|Vector|BreakVector _worlddirection))
  (bind _returnvalue_3 (* (Math|Vector|MakeVector _x _y -14.0) (Math|Vector|MakeVector _returnvalue_2 _returnvalue_2 1.5e+02)))
  (bind _returnvalue_4 (+ _returnvalue_3 _worldlocation))
  (bind _asbottle (Utilities|Casting|CastToBottle (.HitActor (Collision|BreakHitResult (stale Input|MouseEvents|LeftMouseButton _outhit)))))
  (if (not (Variables|/Game/Blueprints/BP_Pouring/Core/Bottle.Bottle_C|GetisPouring _asbottle))
    (if false
      (Physics|Components|PhysicsHandle|SetTargetLocation (Variables|Default|GetPhysicsHandle) _returnvalue_4)
      (elif (Utilities|IsValid _grabedcomponent)
        (Transformation|SetWorldLocation _grabedcomponent (Math|Transform|InverseTransformLocation (Math|Conversions|ToTransform(Vector) (Variables|Default|GetGrabLocation)) _returnvalue_4) false false)
        (if (Utilities|IsValid (stale Input|MouseEvents|LeftMouseButton _asbottle))
          (Default|BottleMoving (stale Input|MouseEvents|LeftMouseButton _asbottle)))))))

(event Input|MouseEvents|LeftMouseButton
  (params (Key :type Key%20Structure :default "None"))
  (bind _returnvalue (Game|GetPlayerController 0))
  (bind _grab_mode (Variables|Default|GetGrab%20Mode))
  (bind (_worldlocation _worlddirection) (Game|Player|ConvertMouseLocationToWorldSpace _returnvalue))
  (:Pressed
    (if _grab_mode
      (bind (_outhit _returnvalue_2) (Collision|LineTraceByChannel _worldlocation (+ (* _worlddirection (Math|Float|MakeLiteralFloat 1e+06)) _worldlocation) "TraceTypeQuery3" true 0 "None"))
      (bind _asbottle (Utilities|Casting|CastToBottle (.HitActor (Collision|BreakHitResult _outhit))))
      (if (Variables|/Game/Blueprints/BP_Pouring/Core/Bottle.Bottle_C|GetDidMove _asbottle)
        _
        (else
          (Variables|/Game/Blueprints/BP_Pouring/Core/Bottle.Bottle_C|SetDidMove _asbottle true)))
      (if _returnvalue_2
        (Variables|Default|SetBottleText (Variables|/Game/Blueprints/BP_Pouring/Core/Bottle.Bottle_C|GetTextRender _asbottle))
        (if (Utilities|Enum|Equal(Enum) (Variables|/Script/Engine.SceneComponent|GetMobility (.HitComponent (Collision|BreakHitResult _outhit))) (Utilities|Enum|LiteralenumEComponentMobility "Movable"))
          (Variables|Default|SetOriginalDistanceToObject (.Distance (Collision|BreakHitResult _outhit)))
          (bind _output_get (Variables|Default|SetGrabedComponent (.HitComponent (Collision|BreakHitResult _outhit))))
          (Utilities|Time|SetTimerbyEvent (delegate Custom|Grabtick) 0.05 true)
          (if (Physics|IsSimulatingPhysics _output_get "None")
            (Class|PhysicsHandleComponent|GrabComponentatLocation (Variables|Default|GetPhysicsHandle) (Variables|Default|GetGrabedComponent) "None" (.Location (Collision|BreakHitResult _outhit)))
            (else
              (Variables|Default|SetGrabLocation (Math|Transform|InverseTransformLocation (Math|Conversions|ToTransform(Vector) (Transformation|GetWorldLocation (.HitComponent (Collision|BreakHitResult _outhit)))) (.Location (Collision|BreakHitResult _outhit))))))))))
  (:Released
    (if _grab_mode
      (Variables|Default|SetGrabedComponent 0)
      (Physics|Components|PhysicsHandle|ReleaseComponent (Variables|Default|GetPhysicsHandle)))))

(fn ConstructionScript)