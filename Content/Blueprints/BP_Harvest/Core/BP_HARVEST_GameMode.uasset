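; Game mode for the Harvest game that shows the main HUD widget and spawns vines ahead of the player.
; On BeginPlay it binds vine-over and spawn-vine events and places the first vine relative to the player pawn.
; A finished vine with no good count left sends the player onward, while spawn requests create and track the next vine.
; In a first game, it quits once the spawn count passes a fixed limit.
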(event Custom|VineOverEvent
  (if (== (Variables|/Game/Blueprints/BP_Harvest/Core/BP_HARVEST_Grapes/BP_HARVEST_Vine.BP_HARVEST_Vine_C|GetGoodCount (Variables|Default|GetCurrentVine)) 0)
    (bind _asbp_harvest_player (Utilities|Casting|CastToBP_HARVEST_Player (Game|Player|GetPlayerPawn 0)))
    (Default|CallGotoNextVine _asbp_harvest_player)))

(event Custom|SpawnVineEvent
  (bind _asbp_harvest_player (Utilities|Casting|CastToBP_HARVEST_Player (Game|Player|GetPlayerPawn 0)))
  (bind _returnvalue (Game|SpawnActorfromClass "/Game/Blueprints/BP_Harvest/Core/BP_HARVEST_Grapes/BP_HARVEST_Vine.BP_HARVEST_Vine_C" (Math|Transform|MakeTransform (Math|Vector|MakeVector (+ (.X (Class|KismetMathLibrary|BreakVector3f (.Location (Math|Transform|BreakTransform (Transformation|GetActorTransform _asbp_harvest_player))))) 722.0 (Variables|Default|GetX_Offset)) (Variables|Default|GetY_PlayerConst) (- (.Z (Class|KismetMathLibrary|BreakVector3f (.Location (Math|Transform|BreakTransform (Transformation|GetActorTransform _asbp_harvest_player))))) 6e+01))) "Undefined" 0 0))
  (Variables|Default|SetCurrentVine _returnvalue)
  (bind _output_get (Variables|Default|SetVinesCreated (+ (Variables|Default|GetVinesCreated) 1)))
  (if (Variables|Default|GetisFirstGame)
    (if (> _output_get 10)
      (Game|QuitGame 0 "Quit" false))))

(event EventBeginPlay
  (bind _returnvalue (UserInterface|CreateWidget "/Game/UI/Harvest_UI/Widgets/HARVEST_Main_WidgetBlueprint.HARVEST_Main_WidgetBlueprint_C"))
  (UserInterface|Viewport|AddtoViewport _returnvalue 0)
  (EventDispatchers|BindEventtoVineOver (delegate Custom|VineOverEvent))
  (EventDispatchers|BindEventtoSpawnVine (delegate Custom|SpawnVineEvent))
  (bind _asbp_harvest_player (Utilities|Casting|CastToBP_HARVEST_Player (Game|Player|GetPlayerPawn 0)))
  (bind _returnvalue_2 (Game|SpawnActorfromClass "/Game/Blueprints/BP_Harvest/Core/BP_HARVEST_Grapes/BP_HARVEST_Vine.BP_HARVEST_Vine_C" (Math|Transform|MakeTransform (Math|Vector|MakeVector (+ (.X (Class|KismetMathLibrary|BreakVector3f (.Location (Math|Transform|BreakTransform (Transformation|GetActorTransform _asbp_harvest_player))))) 2e+02 0.0) (Variables|Default|GetY_PlayerConst) (- (.Z (Class|KismetMathLibrary|BreakVector3f (.Location (Math|Transform|BreakTransform (Transformation|GetActorTransform _asbp_harvest_player))))) 6e+01))) "Undefined" 0 0))
  (Variables|Default|SetCurrentVine _returnvalue_2))

(fn ConstructionScript)