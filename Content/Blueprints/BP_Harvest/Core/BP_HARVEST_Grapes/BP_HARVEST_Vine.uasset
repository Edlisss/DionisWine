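; BP_HARVEST_Vine is a grapevine actor in the harvest game, holding ten grape bunches as child actors.
; On BeginPlay it casts each child to BP_HARVEST_Bunch and tallies those flagged IsGood into GoodCount.
; When a BP_HARVEST_Player begins overlapping it, the vine registers itself as CurrentVine on BP_HARVEST_GameMode.
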(event EventBeginPlay
  (for _array_element (Utilities|Array|MakeArray (Variables|Default|GetBunch1) (Variables|Default|GetBunch2) (Variables|Default|GetBunch3) (Variables|Default|GetBunch4) (Variables|Default|GetBunch5) (Variables|Default|GetBunch6) (Variables|Default|GetBunch7) (Variables|Default|GetBunch8) (Variables|Default|GetBunch9) (Variables|Default|GetBunch10))
    (bind _asbp_harvest_bunch (Utilities|Casting|CastToBP_HARVEST_Bunch (Variables|/Script/Engine.ChildActorComponent|GetChildActor _array_element)))
    (if (Variables|/Game/Blueprints/BP_Harvest/Core/BP_HARVEST_Grapes/BP_HARVEST_Bunch.BP_HARVEST_Bunch_C|GetisGood _asbp_harvest_bunch)
      (Variables|Default|SetGoodCount (+ (Variables|Default|GetGoodCount) 1)))))

(event Collision|EventActorBeginOverlap
  (params (OtherActor :type Actor%20Object%20Reference))
  (Utilities|Casting|CastToBP_HARVEST_Player OtherActor)
  (bind _asbp_harvest_game_mode (Utilities|Casting|CastToBP_HARVEST_GameMode (Game|GetGameMode)))
  (Variables|/Game/Blueprints/BP_Harvest/Core/BP_HARVEST_GameMode.BP_HARVEST_GameMode_C|SetCurrentVine _asbp_harvest_game_mode self))

(fn ConstructionScript)