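; Game mode for a bottle-pouring minigame that runs timed matches, tracks score and quits after the last one.
; On BeginPlay it spawns bottles through BottleSpawnHelper, starts a looping timer and shows the main UI and cursor.
; ScoreUp adds points and uses the remaining Bottle actor count to flag when the next call ends the match.
; EndMatch respawns with one more bottle, or applies a time-based score adjustment before quitting.
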(event Custom|AddTime
  (Variables|Default|SetCurrentTime (+ (Variables|Default|GetCurrentTime) 0.1)))

(event Custom|ScoreUp
  (Variables|Default|SetScore (+ (Variables|Default|GetScore) (Variables|Default|GetScoreAdd)))
  (bind _outactors (Actor|GetAllActorsOfClass "/Game/Blueprints/BP_Pouring/Core/Bottle.Bottle_C"))
  (if (Variables|Default|GetShouldEndMatch)
    (CallFunction|EndMatch)
    (else
      (Variables|Default|SetShouldEndMatch (== (Utilities|Array|Length _outactors) 2))
      (Variables|Default|SetBottleSummary (+ (Variables|Default|GetBottleSummary) (Variables|Default|GetBottleQuantity))))))

(event Custom|EndMatch
  (Development|PrintString "Hello")
  (bind _output_get (Variables|Default|SetCurrentMatch (+ (Variables|Default|GetCurrentMatch) 1)))
  (if (> _output_get (Variables|Default|GetMatchQuantity))
    (bind _output_get_2 (Variables|Default|SetScore (+ (Variables|Default|GetScore) (* (Math|Float|Round (- (* (Variables|Default|GetTimeForBottle) (Variables|Default|GetBottleSummary)) (Variables|Default|GetCurrentTime))) (/ (Variables|Default|GetScoreAdd) 10)))))
    (Development|PrintString (Utilities|String|ToString(Integer) _output_get_2))
    (Game|QuitGame 0 "Quit" false)
    (else
      (bind _output_get_3 (Variables|Default|SetBottleQuantity (+ (Variables|Default|GetBottleQuantity) 1)))
      (bind _returnvalue (Actor|GetActorOfClass "/Game/Blueprints/BP_Pouring/Core/BottleSpawnHelper.BottleSpawnHelper_C"))
      (Default|RefreshSpawn _returnvalue)
      (for _index (range 1 _output_get_3)
        (Default|Spawner _returnvalue))
      (Variables|Default|SetShouldEndMatch false))))

(event EventBeginPlay
  (bind _returnvalue (Actor|GetActorOfClass "/Game/Blueprints/BP_Pouring/Core/BottleSpawnHelper.BottleSpawnHelper_C"))
  (for _index (range 1 (Variables|Default|GetBottleQuantity))
    (Default|Spawner _returnvalue))
  (Variables|/Script/Engine.PlayerController|SetbShowMouseCursor (Game|GetPlayerController 0) true)
  (Utilities|Time|SetTimerbyEvent (delegate Custom|AddTime) 0.1 true)
  (bind _returnvalue_2 (UserInterface|CreateWidget "/Game/UI/Pouring_UI/WBP_PouringMain.WBP_PouringMain_C"))
  (Variables|Default|SetMain%20UI _returnvalue_2)
  (UserInterface|Viewport|AddtoViewport _returnvalue_2 0))

(fn ConstructionScript)