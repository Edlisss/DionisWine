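; Game mode for a rhythm minigame that spawns key widgets on a looping BPM timer while the soundtrack plays, then quits the game when a fixed timer ends.
; Bound events flag an index as pressable when a key is close and handle button presses.
; A valid press raises the streak multiplier, adds streak-scaled score, clears the flag and destroys the last reported key.
; Mistimed presses or break-streak events reset the multiplier.
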(event Custom|ButtonPressedEvent
  (params (Index :type Integer))
  (bind _shouldpressarray (Variables|Default|GetShouldPressArray))
  (bind _output (Utilities|Array|Get(acopy) _shouldpressarray Index))
  (if _output
    (Development|PrintString (Utilities|String|ToString(Boolean) _output))
    (Variables|Default|SetStreak (+ (Variables|Default|GetStreak) 0.01))
    (Variables|Default|SetScore (Math|Conversions|ToInteger(Byte) (+ (Variables|Default|GetScore) (Class|KismetMathLibrary|ToInt64(Float) (* (Variables|Default|GetStreak) 1e+03)))))
    (|SetBy-RefVar _output false)
    (Default|CallDestroy (Variables|Default|GetLast%20Button))
    (else
      (CallFunction|BreakStreakEvent))))

(event Custom|SpawnEvent
  (bind _returnvalue (UserInterface|CreateWidget "/Game/Srgio/PP_MiniGame/Widgets/PP_Key_WidgetBliueprint.PP_Key_WidgetBliueprint_C"))
  (UserInterface|Viewport|AddtoViewport _returnvalue 0))

(event Custom|BreakStreakEvent
  (Variables|Default|SetStreak 1.0))

(event Custom|IsCloseEvent
  (params (Index :type Integer) (Last%20button :type PP%20Key%20Widget%20Bliueprint%20Object%20Reference))
  (Utilities|Array|SetArrayElem (Variables|Default|GetShouldPressArray) Index true)
  (Variables|Default|SetLast%20Button Last%20button))

(event EventBeginPlay
  (EventDispatchers|BindEventtoIsClose (delegate Custom|IsCloseEvent))
  (EventDispatchers|BindEventtoBreakStreak (delegate Custom|BreakStreakEvent))
  (EventDispatchers|BindEventtoButtonPressed (delegate Custom|ButtonPressedEvent))
  (bind _returnvalue (UserInterface|CreateWidget "/Game/Srgio/PP_MiniGame/Widgets/PP_Main_WidgetBlueprint.PP_Main_WidgetBlueprint_C"))
  (bind _output_get (Variables|Default|SetHUD _returnvalue))
  (UserInterface|Viewport|AddtoViewport _output_get 0)
  (Utilities|Time|SetTimerbyEvent (delegate Custom|SpawnEvent) (Variables|Default|GetBPM) true)
  (Utilities|Time|SetTimerbyFunctionName 0 "GameEnd" 266.0)
  (Audio|PlaySound2D "/Game/Srgio/PP_MiniGame/Sound/PP_OST.PP_OST" 1.0 1.0 0.0 0 0))

(fn ConstructionScript)

(fn GameEnd
  (Game|QuitGame 0 "Quit" false))