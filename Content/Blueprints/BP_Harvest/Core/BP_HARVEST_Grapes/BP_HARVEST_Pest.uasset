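; BP_HARVEST_Pest is a pest on a harvest minigame item, likely a grape, that eats it unless removed in time.
; On BeginPlay it binds its DeletePest dispatcher, which clears the parent's pest flag and destroys the pest, and starts a one-shot timer.
; When the timer fires, it decrements the owning vine's GoodCount, calls the GameMode's CallVineOver, then destroys the parent and itself.
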(event Custom|DeletePestEvent
  (Variables|/Game/Blueprints/BP_Harvest/Core/BP_HARVEST_Grapes/BP_HARVEST_Bunch.BP_HARVEST_Bunch_C|SetisWithPest (Variables|Default|GetParent) false)
  (Actor|DestroyActor))

(event Custom|PestAte
  (bind _asbp_harvest_vine (Utilities|Casting|CastToBP_HARVEST_Vine (Actor|GetParentActor (Variables|Default|GetParent))))
  (Variables|/Game/Blueprints/BP_Harvest/Core/BP_HARVEST_Grapes/BP_HARVEST_Vine.BP_HARVEST_Vine_C|SetGoodCount _asbp_harvest_vine (- (Variables|/Game/Blueprints/BP_Harvest/Core/BP_HARVEST_Grapes/BP_HARVEST_Vine.BP_HARVEST_Vine_C|GetGoodCount _asbp_harvest_vine) 1))
  (bind _asbp_harvest_game_mode (Utilities|Casting|CastToBP_HARVEST_GameMode (Game|GetGameMode)))
  (Default|CallVineOver _asbp_harvest_game_mode)
  (Actor|DestroyActor (Variables|Default|GetParent))
  (Actor|DestroyActor))

(event EventBeginPlay
  (EventDispatchers|BindEventtoDeletePest (delegate Custom|DeletePestEvent))
  (Utilities|Time|SetTimerbyEvent (delegate Custom|PestAte) 1e+01))

(fn ConstructionScript)