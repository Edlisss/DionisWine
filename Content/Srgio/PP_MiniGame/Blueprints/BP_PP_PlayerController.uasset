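; Player controller for the PP minigame that turns the four directional inputs into numbered button presses.
; Each press casts to BP_PP_GameMode, reports the direction's index through CallButtonPressed and tells the game mode's HUD to show that button as pressed.
; Each release only tells the HUD to restore that button's image, with no game mode notification.
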(event Input|ActionEvents|InputActionUp
  (params (Key :type Key%20Structure))
  (bind _returnvalue (Game|GetGameMode))
  (:Pressed
    (bind _asbp_pp_game_mode (Utilities|Casting|CastToBP_PP_GameMode _returnvalue))
    (Default|CallButtonPressed _asbp_pp_game_mode)
    (Default|CallPressImage (Variables|/Game/Srgio/PP_MiniGame/Blueprints/BP_PP_GameMode.BP_PP_GameMode_C|GetHUD _asbp_pp_game_mode)))
  (:Released
    (bind _asbp_pp_game_mode_2 (Utilities|Casting|CastToBP_PP_GameMode _returnvalue))
    (Default|CallUnPressImage (Variables|/Game/Srgio/PP_MiniGame/Blueprints/BP_PP_GameMode.BP_PP_GameMode_C|GetHUD _asbp_pp_game_mode_2))))

(event Input|ActionEvents|InputActionDown
  (params (Key :type Key%20Structure))
  (bind _returnvalue (Game|GetGameMode))
  (:Pressed
    (bind _asbp_pp_game_mode (Utilities|Casting|CastToBP_PP_GameMode _returnvalue))
    (Default|CallButtonPressed _asbp_pp_game_mode 1)
    (Default|CallPressImage (Variables|/Game/Srgio/PP_MiniGame/Blueprints/BP_PP_GameMode.BP_PP_GameMode_C|GetHUD _asbp_pp_game_mode) 1))
  (:Released
    (bind _asbp_pp_game_mode_2 (Utilities|Casting|CastToBP_PP_GameMode _returnvalue))
    (Default|CallUnPressImage (Variables|/Game/Srgio/PP_MiniGame/Blueprints/BP_PP_GameMode.BP_PP_GameMode_C|GetHUD _asbp_pp_game_mode_2) 1)))

(event Input|ActionEvents|InputActionLeft
  (params (Key :type Key%20Structure))
  (bind _returnvalue (Game|GetGameMode))
  (:Pressed
    (bind _asbp_pp_game_mode (Utilities|Casting|CastToBP_PP_GameMode _returnvalue))
    (Default|CallButtonPressed _asbp_pp_game_mode 2)
    (Default|CallPressImage (Variables|/Game/Srgio/PP_MiniGame/Blueprints/BP_PP_GameMode.BP_PP_GameMode_C|GetHUD _asbp_pp_game_mode) 2))
  (:Released
    (bind _asbp_pp_game_mode_2 (Utilities|Casting|CastToBP_PP_GameMode _returnvalue))
    (Default|CallUnPressImage (Variables|/Game/Srgio/PP_MiniGame/Blueprints/BP_PP_GameMode.BP_PP_GameMode_C|GetHUD _asbp_pp_game_mode_2) 2)))

(event Input|ActionEvents|InputActionRight
  (params (Key :type Key%20Structure))
  (bind _returnvalue (Game|GetGameMode))
  (:Pressed
    (bind _asbp_pp_game_mode (Utilities|Casting|CastToBP_PP_GameMode _returnvalue))
    (Default|CallButtonPressed _asbp_pp_game_mode 3)
    (Default|CallPressImage (Variables|/Game/Srgio/PP_MiniGame/Blueprints/BP_PP_GameMode.BP_PP_GameMode_C|GetHUD _asbp_pp_game_mode) 3))
  (:Released
    (bind _asbp_pp_game_mode_2 (Utilities|Casting|CastToBP_PP_GameMode _returnvalue))
    (Default|CallUnPressImage (Variables|/Game/Srgio/PP_MiniGame/Blueprints/BP_PP_GameMode.BP_PP_GameMode_C|GetHUD _asbp_pp_game_mode_2) 3)))

(fn ConstructionScript)