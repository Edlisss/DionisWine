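; Game mode for a timed barrel-placement game that runs over successive matches.
; It spawns barrels in rows of six with a timer widget, and a delayed Tick counts down to quit.
; A score dispatcher adds points and ends the match once all barrels are placed.
; EndMatch quits after the last match, otherwise loops over placement spots, clearing each and repeating barrel respawn, count increase and timer reset inside that loop.
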(event Custom|SpawnBarrels
  (bind _initiallocation (Variables|Default|GetInitialLocation))
  (bind _location (Math|Transform|BreakTransform _initiallocation))
  (bind (_x _y _z) (Class|KismetMathLibrary|BreakVector3f _location))
  (if (== (Variables|Default|GetCurrentMatch) 2)
    _
    (else
      (bind _returnvalue (UserInterface|CreateWidget "/Game/UI/AGE_UI/AGE_Timer_W.AGE_Timer_W_C"))
      (UserInterface|Viewport|AddtoViewport _returnvalue 0)))
  (for _index (range 0 (Variables|Default|GetBarrelQauntity))
    (bind _output_get (Variables|Default|SetTempLocation (Math|Transform|MakeTransform (Math|Vector|MakeVector (- _x (* (Math|Float|Floor (/ _index 6)) 200)) (+ (* (Math|Integer|%(Integer) _index 6) 200) _y) _z))))
    (bind _returnvalue_2 (Game|SpawnActorfromClass "/Game/Blueprints/BP_Age/BP_AGE_Barrel.BP_AGE_Barrel_C" _output_get "Undefined" 0 0))
    (Utilities|Array|Add (Variables|Default|GetBarrelArray) _returnvalue_2)))

(event Custom|ScoreUp
  (bind _asbp_age_game_mode (Utilities|Casting|CastToBP_AGE_GameMode (Game|GetGameMode)))
  (Variables|BP_AGE_GameMode_C|SetScore _asbp_age_game_mode (+ (Variables|BP_AGE_GameMode_C|GetScore _asbp_age_game_mode) 100))
  (bind _outactors (Actor|GetAllActorsOfClass "/Game/Blueprints/BP_Age/BP_AGE_Barrel.BP_AGE_Barrel_C"))
  (Variables|Default|SetShouldEndMatch true)
  (for _array_element _outactors
    (Variables|Default|SetShouldEndMatch (and (Variables|/Game/Blueprints/BP_Age/BP_AGE_Barrel.BP_AGE_Barrel_C|GetisPlaced _array_element) (Variables|Default|GetShouldEndMatch)))
    (Development|PrintString "Hello"))
  (Development|PrintString (Utilities|String|ToString(Boolean) (Variables|Default|GetShouldEndMatch)))
  (if (Variables|Default|GetShouldEndMatch)
    (CallFunction|EndMatch)))

(event Custom|EndMatch
  (bind _output_get (Variables|Default|SetCurrentMatch (+ (Variables|Default|GetCurrentMatch) 1)))
  (if (> _output_get (Variables|Default|GetMatchQauntity))
    (Game|QuitGame 0 "Quit" false)
    (else
      (bind _outactors (Actor|GetAllActorsOfClass "/Game/Blueprints/BP_Age/BP_AGE_PlaceForBarrel.BP_AGE_PlaceForBarrel_C"))
      (for _array_element _outactors
        (Variables|/Game/Blueprints/BP_Age/BP_AGE_PlaceForBarrel.BP_AGE_PlaceForBarrel_C|SetisEmpty _array_element true)
        (bind _outactors_2 (Actor|GetAllActorsOfClass "/Game/Blueprints/BP_Age/BP_AGE_Barrel.BP_AGE_Barrel_C"))
        (for _array_element_2 _outactors_2
          (Actor|DestroyActor _array_element_2))
        (Variables|Default|SetBarrelQauntity (+ (Variables|Default|GetBarrelQauntity) (Variables|Default|GetIncrement)))
        (if (> (+ (Variables|Default|GetInitialSeconds) (* (Variables|Default|GetCurrentMatch) 8)) 60)
          (Variables|Default|SetMinutes (+ (Variables|Default|GetInitialMinutes) 1))
          (Variables|Default|SetSeconds (Math|Integer|%(Integer) (+ (Variables|Default|GetInitialSeconds) (* (Variables|Default|GetCurrentMatch) 8)) 60))
          (else
            (Variables|Default|SetSeconds (+ (Variables|Default|GetInitialSeconds) (* (Variables|Default|GetCurrentMatch) 8)))))
        (CallFunction|SpawnBarrels)))))

(event EventBeginPlay
  (CallFunction|SpawnBarrels)
  (EventDispatchers|BindEventtoScoreUpDispatcher (delegate Custom|ScoreUp)))

(event EventTick
  (params (DeltaSeconds :type Float%20%28single-precision%29))
  (Utilities|FlowControl|Delay 1.0)
  (if (== (Variables|Default|GetSeconds) 0)
    (if (== (Variables|Default|GetMinutes) 0)
      (Game|QuitGame 0 "Quit" false)
      (else
        (Variables|Default|SetMinutes (- (Variables|Default|GetMinutes) 1))
        (Variables|Default|SetSeconds 59)))
    (else
      (Variables|Default|SetSeconds (- (Variables|Default|GetSeconds) 1)))))

(fn ConstructionScript)

(fn BarrelCheck
  (Variables|Default|SetTempTypeBarrel true)
  (for _index (range 0 8)
    (Variables|Default|SetTempTypeBarrel (and (<= (Utilities|Array|Get(acopy) (Variables|Default|GetBarrelType) _index) 4) (Variables|Default|GetTempTypeBarrel))))
  (return (Variables|Default|GetTempTypeBarrel)))