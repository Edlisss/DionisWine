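; BP_PouringGameMode is the game mode for the pouring game, running a countdown that quits the game at the target time.
; BeginPlay shows the mouse cursor, starts a looping 0.1-second timer and adds the WBP_PouringMain widget to the viewport.
; Each tick of that timer advances CurrentTime and sends the remaining time to MainUI.
; MainUI is set to None on BeginPlay rather than to the created widget.
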(event Custom|EndGameByTimer
  (Variables|Default|SetCurrentTime (+ (Variables|Default|GetCurrentTime) 0.1))
  (Default|ChangeTimetoEnd (Variables|Default|GetMain%20UI) (- (Variables|Default|GetTargetTime) (Variables|Default|GetCurrentTime)))
  (if (>= (Variables|Default|GetCurrentTime) (Variables|Default|GetTargetTime))
    (Game|QuitGame 0 "Quit" false)))

(event EventBeginPlay
  (Variables|/Script/Engine.PlayerController|SetbShowMouseCursor (Game|GetPlayerController 0) true)
  (Utilities|Time|SetTimerbyEvent (delegate Custom|EndGameByTimer) 0.1 true)
  (bind _returnvalue (UserInterface|CreateWidget "/Game/UI/Pouring_UI/WBP_PouringMain.WBP_PouringMain_C"))
  (Variables|Default|SetMain%20UI 0)
  (UserInterface|Viewport|AddtoViewport _returnvalue 0))

(fn ConstructionScript)