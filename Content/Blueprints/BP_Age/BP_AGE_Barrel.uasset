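; BP_AGE_Barrel is a barrel for the Age game that shows a randomly chosen temperature and years value.
; On BeginPlay it binds and calls its Spawn dispatcher, which rerolls both indices until the game mode's BarrelCheck returns true.
; It then calls SetIndexesEvent, empty here, and applies the matching materials to its Temperature and Years components.
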(event Custom|SetIndexesEvent)

(event Custom|SpawnEvent
  (bind _returnvalue (Math|Random|RandomInteger 3))
  (while (not (Variables|Default|GetisBarrelValid))
    (Variables|Default|SetTemperatureIndex _returnvalue)
    (Variables|Default|SetYearsIndex _returnvalue)
    (bind _asbp_age_game_mode (Utilities|Casting|CastToBP_AGE_GameMode (Game|GetGameMode)))
    (bind _needtorespawn (Default|BarrelCheck _asbp_age_game_mode))
    (Variables|Default|SetisBarrelValid _needtorespawn))
  (CallFunction|SetIndexesEvent)
  (Rendering|Material|SetMaterial (Variables|Default|GetTemperature) 0 (Utilities|Array|Get(acopy) (Variables|Default|GetTemperatureTextures) (Variables|Default|GetTemperatureIndex)))
  (Rendering|Material|SetMaterial (Variables|Default|GetYears) 0 (Utilities|Array|Get(acopy) (Variables|Default|GetYearsTextures) (Variables|Default|GetYearsIndex))))

(event EventBeginPlay
  (EventDispatchers|BindEventtoSpawn (delegate Custom|SpawnEvent))
  (Default|CallSpawn))

(fn ConstructionScript)