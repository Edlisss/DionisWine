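; BP_HARVEST_Bunch is a harvestable grape bunch in the harvest game that randomly spawns good or bad, sometimes guarded by a pest.
; BeginPlay sets the sphere's material by quality, raises it (both random IsUp branches move it up equally) and may spawn a BP_HARVEST_Pest parented to it.
; Harvesting works only without a pest: good bunches add score, decrement the parent vine's count and call CallVineOver; bad ones subtract score.
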(event Custom|HarvestEvent
  (if (not (Variables|Default|GetisWithPest))
    (if (Variables|Default|GetisGood)
      (bind _asbp_harvest_vine (Utilities|Casting|CastToBP_HARVEST_Vine (Actor|GetParentActor)))
      (Variables|/Game/Blueprints/BP_Harvest/Core/BP_HARVEST_Grapes/BP_HARVEST_Vine.BP_HARVEST_Vine_C|SetGoodCount _asbp_harvest_vine (- (Variables|/Game/Blueprints/BP_Harvest/Core/BP_HARVEST_Grapes/BP_HARVEST_Vine.BP_HARVEST_Vine_C|GetGoodCount _asbp_harvest_vine) 1))
      (bind _asbp_harvest_game_mode (Utilities|Casting|CastToBP_HARVEST_GameMode (Game|GetGameMode)))
      (Variables|/Game/Blueprints/BP_Harvest/Core/BP_HARVEST_GameMode.BP_HARVEST_GameMode_C|SetScore _asbp_harvest_game_mode (+ (Variables|/Game/Blueprints/BP_Harvest/Core/BP_HARVEST_GameMode.BP_HARVEST_GameMode_C|GetScore _asbp_harvest_game_mode) 5e+02))
      (Default|CallVineOver _asbp_harvest_game_mode)
      (Actor|DestroyActor)
      (else
        (bind _asbp_harvest_game_mode_2 (Utilities|Casting|CastToBP_HARVEST_GameMode (Game|GetGameMode)))
        (Variables|/Game/Blueprints/BP_Harvest/Core/BP_HARVEST_GameMode.BP_HARVEST_GameMode_C|SetScore _asbp_harvest_game_mode_2 (- (Variables|/Game/Blueprints/BP_Harvest/Core/BP_HARVEST_GameMode.BP_HARVEST_GameMode_C|GetScore _asbp_harvest_game_mode_2) 5e+02))
        (Actor|DestroyActor)))))

(event EventBeginPlay
  (bind _sphere (Variables|Default|GetSphere))
  (bind _sphere_2 (Variables|Default|GetSphere))
  (bind _returnvalue (Transformation|GetWorldLocation _sphere))
  (bind (_x _y _z) (Class|KismetMathLibrary|BreakVector3f _returnvalue))
  (EventDispatchers|BindEventtoHarvest (delegate Custom|HarvestEvent))
  (bind _output_get (Variables|Default|SetisUp (Math|Random|RandomBool)))
  (bind _output_get_2 (Variables|Default|SetisGood (> (Math|Random|RandomFloat) 0.2)))
  (if _output_get
    (Transformation|SetWorldLocation _sphere (Math|Vector|MakeVector _x _y (+ _z 4e+01)) false false)
    (else
      (Transformation|SetWorldLocation _sphere (Math|Vector|MakeVector _x _y (- _z -4e+01)) false false)))
  (if _output_get_2
    (Rendering|Material|SetMaterial _sphere_2 0 "/Game/Models/Material/Harvest_Materials/M_GoodBunch.M_GoodBunch")
    (else
      (Rendering|Material|SetMaterial _sphere_2 0 "/Game/Models/Material/Harvest_Materials/M_BadBunc.M_BadBunc")))
  (bind _output_get_3 (Variables|Default|SetisWithPest (<= (Math|Random|RandomFloat) 0.4)))
  (if _output_get_3
    (bind _returnvalue_2 (Game|SpawnActorfromClass "/Game/Blueprints/BP_Harvest/Core/BP_HARVEST_Grapes/BP_HARVEST_Pest.BP_HARVEST_Pest_C" (Transformation|GetActorTransform) "Undefined" 0 0))
    (Variables|/Game/Blueprints/BP_Harvest/Core/BP_HARVEST_Grapes/BP_HARVEST_Pest.BP_HARVEST_Pest_C|SetParent _returnvalue_2 self)))

(fn ConstructionScript)